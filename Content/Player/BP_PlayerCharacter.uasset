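; BP_PlayerCharacter is the player character Blueprint, which puts the HUD on screen when play begins.
; BeginPlay calls a SetupHUD event that checks the HUDWidget class is valid, creates the widget for the local viewing player controller, stores it in HUDReference and adds it to the viewport.
; The construction script is empty, and the graphs contain no other gameplay logic.
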(event `self.ReceiveBeginPlay`
  (`self.SetupHUD`))

(event `SetupHUD`
  (if (`KismetSystemLibrary.IsValidClass` (`self.HUDWidget`))
    (bind _returnvalue (`|CreateWidget` (`self.HUDWidget`) (`self.GetLocalViewingPlayerController` self)))
    (bind _output_get (set `self.HUDReference` _returnvalue))
    (`UserWidget.AddToViewport` _output_get 0)))

(fn `UserConstructionScript`)